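; BP_BALL is a ball actor that moves at a set speed and bounces off whatever blocks it.
; Each Tick it moves by a swept world offset along DIRECTION times SPEED, scaled by delta time.
; On a blocking hit it reflects DIRECTION about the surface normal and zeroes Z to stay horizontal.
; BeginPlay derives DECELERATION from SPEED, but the logic that would slow the ball toward MinSpeed is disconnected.
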(event `self.ReceiveBeginPlay`
  (set `self.DECELERATION` (* (`self.SPEED`) 0.1)))

(event `self.ReceiveTick`
  (params (DeltaSeconds :type "Float (single-precision)"))
  (bind _sweephitresult (`self.K2_AddActorWorldOffset` (* (* (`self.DIRECTION`) (`self.SPEED`)) DeltaSeconds) true))
  (bind (_bblockinghit _binitialoverlap _time _distance _location _impactpoint _normal) (`GameplayStatics.BreakHitResult` _sweephitresult))
  (if _bblockinghit
    (bind (_returnvalue_x _returnvalue_y) (`KismetMathLibrary.BreakVector` (`KismetMathLibrary.GetReflectionVector` (`self.DIRECTION`) _normal)))
    (set `self.DIRECTION` (`KismetMathLibrary.MakeVector` _returnvalue_x _returnvalue_y))))

(fn `UserConstructionScript`)